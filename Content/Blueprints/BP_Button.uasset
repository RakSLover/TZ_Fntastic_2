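; BP_Button is a button Blueprint that spawns a turtle for its current nest when its ButtonPressed event fires.
; The event switches on the nest's NestId to pick one of three turtle classes and spawns it at the nest's location.
; Each turtle receives the nest's start and destination points as spawn parameters.
; The SpawnTurtle function and construction script are empty, so all logic lives in the event graph.
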(event `Event_ButtonPressed`
  (bind _currentnest (`self.CurrentNest`))
  (bind _currentnest_2 (`self.CurrentNest`))
  (bind _currentnest_3 (`self.CurrentNest`))
  (switch `int` (`/Game/Blueprints/BP_Nest.NestId` (`self.CurrentNest`))
    (:`0`
      (`|SpawnActorFromClass` "/Game/Blueprints/BP_Turtle1.BP_Turtle1_C" (`KismetMathLibrary.MakeTransform` (`self.K2_GetActorLocation` _currentnest)) "Undefined" "OverrideRootScale" null (`/Game/Blueprints/BP_Nest.StartPoint` _currentnest) (`/Game/Blueprints/BP_Nest.DestPoint` _currentnest) null))
    (:`1`
      (`|SpawnActorFromClass` "/Game/Blueprints/BP_Turtle2.BP_Turtle2_C" (`KismetMathLibrary.MakeTransform` (`self.K2_GetActorLocation` _currentnest_3)) "Undefined" "OverrideRootScale" null (`/Game/Blueprints/BP_Nest.StartPoint` _currentnest_3) (`/Game/Blueprints/BP_Nest.DestPoint` _currentnest_3) null))
    (:`2`
      (`|SpawnActorFromClass` "/Game/Blueprints/BP_Turtle3.BP_Turtle3_C" (`KismetMathLibrary.MakeTransform` (`self.K2_GetActorLocation` _currentnest_2)) "Undefined" "OverrideRootScale" null (`/Game/Blueprints/BP_Nest.StartPoint` _currentnest_2) (`/Game/Blueprints/BP_Nest.DestPoint` _currentnest_2) null))))

(fn `SpawnTurtle`)

(fn `UserConstructionScript`)