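; BP_Turtle2 is a turtle character that travels toward an EndPoint actor in a stop-and-go rhythm.
; The Move event issues an AI MoveTo, halts the movement component after a short delay, pauses, then reissues the order while GetInMovement returns true.
; A successful move stops the character and calls Finish.
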(event `self.Move`
  (`|AIMoveTo` self (0.0 0.0 0.0) (`self.EndPoint`) 100.0 true :!label _label
    (:`then`
      (`KismetSystemLibrary.Delay` 1.0)
      (`NavMovementComponent.StopActiveMovement` (`self.CharacterMovement`))
      (`KismetSystemLibrary.Delay` 0.5)
      (if (`self.GetInMovement`)
        (goto _label)))
    (:`OnSuccess`
      (`NavMovementComponent.StopActiveMovement` (`self.CharacterMovement`))
      (`self.Finish`))))

(fn `UserConstructionScript`)