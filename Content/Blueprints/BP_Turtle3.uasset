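; Turtle pawn that advances toward an EndPoint in a back-and-forth pattern, using AI movement.
; Move starts AIMoveTo to EndPoint, then redirects to StartPoint after a longer delay and loops after a shorter one while GetInMovement holds.
; The delays run from the immediate exec pin, so each new move interrupts the last.
; Reaching EndPoint stops movement, calls Finish and sets IsFullCompleted, which blocks further retreats.
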(event `self.Move`
  (`|AIMoveTo` self (0.0 0.0 0.0) (`self.EndPoint`) 100.0 :!label _label
    (:`then`
      (`KismetSystemLibrary.Delay` 1.0)
      (if (not (`self.isFullCompleted?`))
        (`|AIMoveTo` self (0.0 0.0 0.0) (`self.StartPoint`)
          (:`then`
            (`KismetSystemLibrary.Delay` 0.5)
            (if (`self.GetInMovement`)
              (goto _label))))))
    (:`OnSuccess`
      (`NavMovementComponent.StopActiveMovement` (`self.CharacterMovement`))
      (`self.Finish`)
      (set `self.isFullCompleted?` true))))

(fn `UserConstructionScript`)